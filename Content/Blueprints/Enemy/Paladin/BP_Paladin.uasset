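; Paladin enemy Blueprint that adds a shield and debug visuals to the logic inherited from its parent class.
; The construction script attaches the Shield component to the mesh's left-hand socket, then runs the parent's construction script.
; Tick draws an inner and an outer debug sphere around the actor, calling parent Tick both before and after with zero delta time.
; BeginPlay and overlap events are disabled placeholder nodes.
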(event EventBeginPlay)

(event Collision|EventActorBeginOverlap
  (params (OtherActor :type Actor%20Object%20Reference))
  (|CallParentFunction OtherActor) ; 此节点被禁用，将不会被调用。\n从引脚连出引线来编译功能。
)

(event EventTick
  (params (DeltaSeconds :type Float%20%28single-precision%29))
  (|CallParentFunction 0.0)
  (Rendering|Debug|DrawDebugSphere (Transformation|GetActorLocation) 2e+02 12 "(R=1.000000,G=1.000000,B=1.000000,A=1.000000)" 0.0)
  (Rendering|Debug|DrawDebugSphere (Transformation|GetActorLocation) 1e+03 12 "(R=1.000000,G=0.000000,B=0.035091,A=1.000000)" 0.0)
  (|CallParentFunction 0.0))

(fn ConstructionScript
  (Transformation|AttachComponentToComponent (Variables|Default|GetShield) (Variables|Character|GetMesh) "LeftHandSocket" "KeepRelative" "KeepRelative" "KeepRelative" true)
  (|CallParentFunction))